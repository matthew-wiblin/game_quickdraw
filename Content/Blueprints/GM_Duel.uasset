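; GM_Duel is the game mode for a samurai quick-draw duel between a player and an NPC.
; Tick moves the phase from Intro to Wait, then after a random delay to Draw, broadcasting the draw start and showing an exclamation actor.
; A successful attack defeats the opponent, hides the exclamation and starts a restart timer.
; Separate functions set the Finish phase and reset both samurai and the round state.
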(event `self.ReceiveBeginPlay`
  (bind _returnvalue (`GameplayStatics.GetActorOfClass` "/Game/Blueprints/BP_Exclamation.BP_Exclamation_C"))
  (set `self.Exclamation_ref` _returnvalue)
  (bind _returnvalue_2 (`GameplayStatics.GetActorOfClass` "/Game/Blueprints/BP_Samurai_player.BP_Samurai_player_C"))
  (set `self.SamuraiPlayer` _returnvalue_2)
  (bind _returnvalue_3 (`GameplayStatics.GetActorOfClass` "/Game/Blueprints/BP_Samurai_NPC.BP_Samurai_NPC_C"))
  (set `self.SamuraiNPC` _returnvalue_3))

(event `self.ReceiveTick`
  (params (DeltaSeconds :type "Float (single-precision)"))
  (set `self.ElapsedTime` (+ DeltaSeconds (`self.ElapsedTime`)))
  (switch `/Game/Blueprints/Enums/E_Phase` (`self.phase`)
    (:`NewEnumerator0`
      (if (>= (`self.ElapsedTime`) (`self.RoundStartTime`))
        (set `self.phase` "NewEnumerator1")
        (`KismetSystemLibrary.Delay` (`KismetMathLibrary.RandomFloatInRange` (`self.MinDrawDelay`) (`self.MaxDrawDelay`)))
        (set `self.phase` "NewEnumerator2")
        (`self.DrawPhaseStarted`)
        (`/Engine/EditorBlueprintResources/StandardMacros.IsValid` (`self.Exclamation_ref`)
          (:`Is Valid`
            (`/Game/Blueprints/BP_Exclamation.SetVisibility` (`self.Exclamation_ref`) true)))))))

(fn `AttackedSuccssfully`
  (params (`Is Player` :type Boolean))
  (if `Is Player`
    (`/Game/Blueprints/BP_Samurai.Defeated` (`self.SamuraiNPC`))
    (else
      (`/Game/Blueprints/BP_Samurai.Defeated` (`self.SamuraiPlayer`))))
  (`/Engine/EditorBlueprintResources/StandardMacros.IsValid` (`self.Exclamation_ref`)
    (:`Is Valid`
      (`/Game/Blueprints/BP_Exclamation.SetVisibility` (`self.Exclamation_ref`) false)
      (`KismetSystemLibrary.K2_SetTimerDelegate` (`|CreateDelegate` :!event `Reset`) (`self.RestartDelay`)))))

(fn `Reset`
  (set `self.phase` "NewEnumerator0")
  (set `self.ElapsedTime` 0.0)
  (`/Game/Blueprints/BP_Samurai.Reset` (`self.SamuraiPlayer`))
  (`/Game/Blueprints/BP_Samurai.Reset` (`self.SamuraiNPC`)))

(fn `SetGameFinished`
  (set `self.phase` "NewEnumerator3"))

(fn `UserConstructionScript`)